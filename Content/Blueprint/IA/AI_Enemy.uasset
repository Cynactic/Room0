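; AI controller for enemies that runs the BT_Enemy behavior tree and feeds it information about the player.
; On BeginPlay it stores the blackboard and a reference to the player's BP_ThirdPersonCharacter.
; Perception updates and Tick share one path writing the player's location and Cacher flag to the blackboard, so values refresh every frame regardless of perception.
; The target-forgotten and Find events are empty stubs.
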(event OnPerceptionUpdated(AIPerception)
  (params (UpdatedActors :type Array%20of%20Actor%20Object%20References))
  (bind _newvar (Variables|Default|GetNewVar))
  (AI|Components|Blackboard|SetValueasVector _newvar (Utilities|Name|MakeLiteralName "PlayerPosition") (Transformation|GetActorLocation (Game|Player|GetPlayerPawn 0)))
  (AI|Components|Blackboard|SetValueasBool _newvar (Utilities|Name|MakeLiteralName "Cacher") (Variables|/Game/ThirdPerson/Blueprints/BP_ThirdPersonCharacter.BP_ThirdPersonCharacter_C|GetCacher? (Variables|Default|GetAs%20BP%20Third%20Person%20Character))))

(event OnTargetPerceptionForgotten(AIPerception)
  (params (Actor :type Actor%20Object%20Reference)))

(event Custom|Find)

(event EventBeginPlay
  (bind _returnvalue (AI|GetBlackboard 0))
  (AI|RunBehaviorTree "/Game/Blueprint/IA/BT_Enemy.BT_Enemy")
  (Variables|Default|SetNewVar _returnvalue)
  (Development|PrintString (Utilities|GetDisplayName _returnvalue))
  (bind _asbp_third_person_character (Utilities|Casting|CastToBP_ThirdPersonCharacter (Game|Player|GetPlayerPawn 0)))
  (Variables|Default|SetAs%20BP%20Third%20Person%20Character _asbp_third_person_character))

(event EventTick
  (params (DeltaSeconds :type Float%20%28single-precision%29))
  (bind _newvar (Variables|Default|GetNewVar))
  (AI|Components|Blackboard|SetValueasVector _newvar (Utilities|Name|MakeLiteralName "PlayerPosition") (Transformation|GetActorLocation (Game|Player|GetPlayerPawn 0)))
  (AI|Components|Blackboard|SetValueasBool _newvar (Utilities|Name|MakeLiteralName "Cacher") (Variables|/Game/ThirdPerson/Blueprints/BP_ThirdPersonCharacter.BP_ThirdPersonCharacter_C|GetCacher? (Variables|Default|GetAs%20BP%20Third%20Person%20Character))))

(fn ConstructionScript)
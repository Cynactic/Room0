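; BP_Enemy is an enemy pawn that turns PawnSensing sightings of the player into calls on its AI_Enemy controller.
; Distant sightings report something in sight and slow the sensing interval, while close ones trigger a chase and speed it up.
; MemoryTimer counts distant sightings rather than elapsed time, resetting on a close one; a high count at longer range sets the controller's AIState to its NewEnumerator0 value.
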(event OnSeePawn(PawnSensing)
  (params (Pawn :type Pawn%20Object%20Reference))
  (bind _returnvalue (Transformation|GetActorLocation))
  (bind _as_bp_third_person_character (Variables|Default|GetAs%20BP%20Third%20Person%20Character))
  (bind _as_ai_enemy (Variables|Default|GetAs%20AI%20Enemy))
  (bind _returnvalue_2 (Transformation|GetActorLocation _as_bp_third_person_character))
  (bind _returnvalue_3 (Math|Vector|Distance(Vector) _returnvalue_2 _returnvalue))
  (bind _returnvalue_4 (>= _returnvalue_3 1e+03))
  (if (== Pawn (Game|Player|GetPlayerPawn 0))
    (Class|PawnSensingComponent|SetSensingInterval (Variables|Default|GetPawnSensing) (Math|Float|SelectFloat 1.0 0.1 _returnvalue_4))
    (if _returnvalue_4
      (Default|CallSomethinginSight (Variables|Default|GetAs%20AI%20Enemy))
      (bind _timeelapsed (CallFunction|Timer))
      (if (and (>= _timeelapsed 5.0) (>= _returnvalue_3 2e+03))
        (Variables|/Game/Blueprint/IA/AI_Enemy.AI_Enemy_C|SetAIState _as_ai_enemy "NewEnumerator0"))
      (else
        (Variables|Default|SetMemory%20Timer 0.0)
        (Default|CallPlayerChase _as_ai_enemy)
        (Development|PrintString "CHASE" true true "(R=1.000000,G=0.068380,B=0.000000,A=1.000000)" 5.0)))))

(event EventBeginPlay
  (bind _asai_enemy (Utilities|Casting|CastToAI_Enemy (Pawn|GetController)))
  (Variables|Default|SetAs%20AI%20Enemy _asai_enemy)
  (bind _asbp_third_person_character (Utilities|Casting|CastToBP_ThirdPersonCharacter (Game|Player|GetPlayerPawn 0)))
  (Variables|Default|SetAs%20BP%20Third%20Person%20Character _asbp_third_person_character))

(event Collision|EventActorBeginOverlap
  (params (OtherActor :type Actor%20Object%20Reference)))

(event EventTick
  (params (DeltaSeconds :type Float%20%28single-precision%29)))

(fn ConstructionScript)

(fn Timer
  (bind _output_get (Variables|Default|SetMemory%20Timer (+ (Variables|Default|GetMemory%20Timer) 1.0)))
  (return _output_get))
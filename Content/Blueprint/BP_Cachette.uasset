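; BP_Cachette is a hiding spot with two doors that sets the player's Cacher (hidden) flag.
; OnInteract alternates between opening and closing the doors, swinging both in opposite directions with the OverturePorte timeline.
; The Box overlap sets Cacher and enables Tick on entry, then clears and disables both on exit.
; While enabled, Tick keeps Cacher true only while the doors are closed.
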(event OnComponentBeginOverlap(Box)
  (params (OverlappedComponent :type Primitive%20Component%20Object%20Reference) (OtherActor :type Actor%20Object%20Reference) (OtherComp :type Primitive%20Component%20Object%20Reference) (OtherBodyIndex :type Integer) (bFromSweep :type Boolean) (SweepResult :type Hit%20Result%20Structure%20%28by%20ref%29))
  (if (== OtherActor (Game|Player|GetPlayerPawn 0))
    (Actor|Tick|SetActorTickEnabled true)
    (Variables|/Game/ThirdPerson/Blueprints/BP_ThirdPersonCharacter.BP_ThirdPersonCharacter_C|SetCacher? (Variables|Default|GetRef_Player) true)))

(event OnComponentEndOverlap(Box)
  (params (OverlappedComponent :type Primitive%20Component%20Object%20Reference) (OtherActor :type Actor%20Object%20Reference) (OtherComp :type Primitive%20Component%20Object%20Reference) (OtherBodyIndex :type Integer))
  (if (== OtherActor (Game|Player|GetPlayerPawn 0))
    (Actor|Tick|SetActorTickEnabled false)
    (Variables|/Game/ThirdPerson/Blueprints/BP_ThirdPersonCharacter.BP_ThirdPersonCharacter_C|SetCacher? (Variables|Default|GetRef_Player) false)))

(event EventBeginPlay
  (bind _asbp_third_person_character (Utilities|Casting|CastToBP_ThirdPersonCharacter (Game|Player|GetPlayerPawn 0)))
  (Variables|Default|SetRef_Player _asbp_third_person_character))

(event EventTick
  (params (DeltaSeconds :type Float%20%28single-precision%29))
  ;[0.15 0.15 0.15 0.5] Une fois caché la cachett effectue une vérification continuelle pour voir si le joueur est caché
  (for _array_element (Collision|GetOverlappingActors (Variables|Default|GetBox) 0 :!class /Script/Engine.PrimitiveComponent)
    (if (!= _array_element self)
      (if (not (Variables|Default|GetPorteOuverte))
        (Variables|/Game/ThirdPerson/Blueprints/BP_ThirdPersonCharacter.BP_ThirdPersonCharacter_C|SetCacher? (Variables|Default|GetRef_Player) true)
        (else
          (Variables|/Game/ThirdPerson/Blueprints/BP_ThirdPersonCharacter.BP_ThirdPersonCharacter_C|SetCacher? (Variables|Default|GetRef_Player) false))))))

(event EventOnInteract
  ;[0.15 0.15 0.15 0.5] Ouverture et fermeture des porte
  (Utilities|FlowControl|FlipFlop
    (:A
      (Variables|Default|SetPorteOuverte true)
      (bind _angleporte (Timeline|OverturePorte PlayFromStart)
        (:Update
          (Transformation|SetRelativeRotation (Variables|Default|GetSM_Porte1) (Math|Rotator|MakeRotator 0.0 0.0 (* _angleporte 9e+01)) false false)
          (Transformation|SetRelativeRotation (Variables|Default|GetSM_Porte) (Math|Rotator|MakeRotator 0.0 0.0 (* (* _angleporte 9e+01) -1.0)) false false))))
    (:B
      (Variables|Default|SetPorteOuverte false)
      (Timeline|OverturePorte Reverse))))

(fn ConstructionScript)
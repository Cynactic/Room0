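; BP_PointSpawn is a spawn point that respawns a pickable, either a battery or a wooden plank depending on TypeSpawner, after a delay.
; Its LancerTimer dispatcher triggers TimerReaparition, which opens a gate on Tick only for the first spawner type.
; Tick accumulates time until TempsDeRespawn, spawns the pickable at its location with itself as owner, then resets and closes the gate.
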(event Custom|ResetTime
  (Variables|Default|SetTimer 0.0)
  ;[0.15 0.15 0.15 0.5] lance et stop le timer de respawn
  (Utilities|FlowControl|Gate true) ; enters at Close
)

(event Custom|TimerReaparition
  (if (== (Variables|Default|GetTypeSpawner) 0)
    ;[0.15 0.15 0.15 0.5] lance et stop le timer de respawn
    (Utilities|FlowControl|Gate true) ; enters at Open
  ))

(event EventBeginPlay
  (EventDispatchers|BindEventtoLancerTimer (delegate Custom|TimerReaparition)))

(event Collision|EventActorBeginOverlap
  (params (OtherActor :type Actor%20Object%20Reference)))

(event EventTick
  (params (DeltaSeconds :type Float%20%28single-precision%29))
  ;[0.15 0.15 0.15 0.5] lance et stop le timer de respawn
  (Utilities|FlowControl|Gate true
    (:Exit
      (bind _output_get (Variables|Default|SetTimer (+ DeltaSeconds (Variables|Default|GetTimer))))
      (if (>= _output_get (Variables|Default|GetTempsDeRespawn))
        ;[0.15 0.15 0.15 0.5] Respawn un objet qui était initialement là
        (Game|SpawnActorfromClass (Utilities|Select :Index (Variables|Default|GetTypeSpawner) :NewEnumerator0 "/Game/Blueprint/Pickable/BP_Pile.BP_Pile_C" :NewEnumerator1 "/Game/Blueprint/Pickable/BP_Planche.BP_Planche_C") (Math|Transform|MakeTransform (Transformation|GetActorLocation) "0, 0, 0" "1.000000,1.000000,1.000000") "AdjustIfPossibleButAlwaysSpawn" "MultiplyWithRoot" self)
        (CallFunction|ResetTime)))))

(fn ConstructionScript
  (switch Utilities|FlowControl|Switch|SwitchonENUM_TypePickable (Variables|Default|GetTypeSpawner)))
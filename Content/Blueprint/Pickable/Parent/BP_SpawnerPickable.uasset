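; BP_SpawnerPickable is a spawner that places battery (BP_Pile) and wooden plank (BP_Planche) pickups in the level.
; On BeginPlay, it clears both lists, then spawns a pickup at every BP_PointSpawn, choosing the class from that point's TypeSpawner and making the point its owner.
; Spawned actors are kept in separate ListPile and ListPlanche lists.
; The ObjetRamasser event and AjouterPointSpawn function are empty stubs.
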(event Custom|ObjetRamasser)

(event EventBeginPlay
  (Utilities|Array|Clear (Variables|Default|GetListPlanche))
  (Utilities|Array|Clear (Variables|Default|GetListPile))
  ;[0.15 0.15 0.15 0.5] Récupère tout les points de spawning et spawn les objets en conséquences
  (bind _outactors (Actor|GetAllActorsOfClass "/Game/Blueprint/Pickable/BP_PointSpawn.BP_PointSpawn_C"))
  (for _array_element _outactors
    (bind _returnvalue (Game|SpawnActorfromClass (Utilities|Select :Index (Variables|/Game/Blueprint/Pickable/BP_PointSpawn.BP_PointSpawn_C|GetTypeSpawner _array_element) :NewEnumerator0 "/Game/Blueprint/Pickable/BP_Pile.BP_Pile_C" :NewEnumerator1 "/Game/Blueprint/Pickable/BP_Planche.BP_Planche_C") (Math|Transform|MakeTransform (Transformation|GetActorLocation _array_element) "0, 0, 0" "1.000000,1.000000,1.000000") "AdjustIfPossibleButAlwaysSpawn" "MultiplyWithRoot" _array_element 0))
    ;[0.15 0.15 0.15 0.5] Conserve dans des listes les piles et planches
    (Utilities|Array|AddUnique (Utilities|Select :Index (Variables|/Game/Blueprint/Pickable/BP_PointSpawn.BP_PointSpawn_C|GetTypeSpawner _array_element) :NewEnumerator0 (Variables|Default|GetListPile) :NewEnumerator1 (Variables|Default|GetListPlanche)) _returnvalue)))

(event Collision|EventActorBeginOverlap
  (params (OtherActor :type Actor%20Object%20Reference)))

(event EventTick
  (params (DeltaSeconds :type Float%20%28single-precision%29)))

(fn ConstructionScript)

(fn AjouterPointSpawn)
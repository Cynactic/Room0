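; Base Blueprint for pickable items, with a battery or wooden plank mesh chosen by type in the construction script.
; At BeginPlay it stores its owning BP_PointSpawn.
; On interaction by the player character, it runs ExecuteAction, empty here, tells the spawn point to start its respawn timer, then destroys itself.
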(event EventBeginPlay
  (bind _asbp_point_spawn (Utilities|Casting|CastToBP_PointSpawn (Components|GetOwner)))
  (Variables|Default|SetParent _asbp_point_spawn))

(event Collision|EventActorBeginOverlap
  (params (OtherActor :type Actor%20Object%20Reference)))

(event EventTick
  (params (DeltaSeconds :type Float%20%28single-precision%29)))

(event EventOnInteract
  (Utilities|Casting|CastToBP_ThirdPersonCharacter (Game|Player|GetPlayerPawn 0))
  ;[0.15 0.15 0.15 0.5] Lance l'action conséquente
  (CallFunction|ExecuteAction)
  ;[0.15 0.15 0.15 0.5] Lance le timer de réaparition
  (Default|CallLancerTimer (Variables|Default|GetParent))
  ;[0.15 0.15 0.15 0.5] Détruit l'objet récupéré
  (Actor|DestroyActor))

(event EventIsPickable
  (params (CanBePicked :type Boolean)))

(fn ConstructionScript
  (switch Utilities|FlowControl|Switch|SwitchonENUM_TypePickable (Variables|Default|GetTypePickable)
    (:NewEnumerator0
      (Components|StaticMesh|SetStaticMesh (Variables|Default|GetPickable) "/Game/Meshes/Pickables/SM_Pile.SM_Pile"))
    (:NewEnumerator1
      (Components|StaticMesh|SetStaticMesh (Variables|Default|GetPickable) "/Game/Meshes/Pickables/SM_Planche001.SM_Planche001"))))

(fn ExecuteAction)
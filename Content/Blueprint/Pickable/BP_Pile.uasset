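; BP_Pile is a battery pickup that the player character collects.
; Its construction script sets the inherited pickable type, then runs the parent's construction script.
; ExecuteAction casts the player pawn to BP_ThirdPersonCharacter, calls TakeBatterie on it, prints a debug message and destroys the pickup.
; The event graph holds only disabled default events.
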(event EventBeginPlay
  (|CallParentFunction) ; This node is disabled and will not be called.\nDrag off pins to build functionality.
)

(event Collision|EventActorBeginOverlap
  (params (OtherActor :type Actor%20Object%20Reference))
  (|CallParentFunction OtherActor) ; This node is disabled and will not be called.\nDrag off pins to build functionality.
)

(event EventTick
  (params (DeltaSeconds :type Float%20%28single-precision%29))
  (|CallParentFunction DeltaSeconds) ; This node is disabled and will not be called.\nDrag off pins to build functionality.
)

(fn ConstructionScript
  (Variables|Default|SetTypePickable "NewEnumerator0")
  (|CallParentFunction))

(fn ExecuteAction
  (bind _asbp_third_person_character (Utilities|Casting|CastToBP_ThirdPersonCharacter (Game|Player|GetPlayerPawn 0)))
  (Default|TakeBatterie _asbp_third_person_character)
  (Development|PrintString "Battery" true true "(R=1.000000,G=0.798187,B=0.000000,A=1.000000)")
  (Actor|DestroyActor))
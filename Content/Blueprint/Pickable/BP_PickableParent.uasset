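; Base Blueprint for pickable items that the player collects by interacting with them.
; The construction script sets the Pickable mesh from the TypePickable value, either a battery or a wooden plank.
; OnInteract checks that player 0's pawn is BP_ThirdPersonCharacter, calls ExecuteAction, then destroys the actor.
; ExecuteAction is empty here, serving as a hook for child Blueprints.
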(event EventBeginPlay)

(event Collision|EventActorBeginOverlap
  (params (OtherActor :type Actor%20Object%20Reference)))

(event EventTick
  (params (DeltaSeconds :type Float%20%28single-precision%29)))

(event EventOnInteract
  (Utilities|Casting|CastToBP_ThirdPersonCharacter (Game|Player|GetPlayerPawn 0))
  (CallFunction|ExecuteAction)
  (Actor|DestroyActor))

(fn ConstructionScript
  (switch Utilities|FlowControl|Switch|SwitchonENUM_TypePickable (Variables|Default|GetTypePickable)
    (:NewEnumerator0
      (Components|StaticMesh|SetStaticMesh (Variables|Default|GetPickable) "/Game/Meshes/Pickables/SM_Pile.SM_Pile"))
    (:NewEnumerator1
      (Components|StaticMesh|SetStaticMesh (Variables|Default|GetPickable) "/Game/Meshes/Pickables/SM_Planche001.SM_Planche001"))))

(fn ExecuteAction)